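; Shopping list component that tracks which items from a data table have been checked off.
; On BeginPlay it collects the table's row names and builds a name-to-bool checklist, all unchecked.
; Checking a listed item by name marks it true, fires an item-checked dispatcher and runs a completion check.
; That check is unfinished: its loop never detects unchecked items, and its only output is a placeholder debug print.
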(event Custom|CreateList
  (for _array_element (Variables|Default|GetAllItems)
    (Utilities|Map|Add (Variables|Default|GetItemsChecklist) _array_element false)))

(event Custom|TryCheckItemFromList
  (params (ItemToCheck :type Struct%20Item%20Structure))
  (bind _itemname (Utilities|Struct|BreakStruct_Item ItemToCheck))
  (bind _itemschecklist (Variables|Default|GetItemsChecklist))
  ;[1 1 1] Check if item is inside the list
  (if (Utilities|Map|Contains _itemschecklist _itemname)
    (Utilities|Map|Add _itemschecklist _itemname true)
    (Default|CallOnItemCheckedOftheList ItemToCheck)
    (CallFunction|CheckforCompletion)))

(event Custom|CheckForCompletion
  (bind _array_element (Utilities|Array|ForEachLoopwithBreak (Variables|Default|GetAllItems) :!label _label)
    (:LoopBody
      (if (.Value (Utilities|Map|Find (Variables|Default|GetItemsChecklist) _array_element))
        (if (not (.ReturnValue (Utilities|Map|Find (Variables|Default|GetItemsChecklist) _array_element)))
          (goto _label Break))))
    (:Completed
      (Development|PrintString "Hello"))))

(event EventBeginPlay
  (Utilities|FlowControl|Sequence
    (:then_0
      ;[1 1 1] Get All elements from the DT
      (bind _outrownames (DataTable|GetDataTableRowNames (Variables|Default|GetItemsDataTableRef)))
      (for _array_element _outrownames
        (Utilities|Array|AddUnique (Variables|Default|GetAllItems) _array_element)))
    (:then_1
      (CallFunction|CreateList))))