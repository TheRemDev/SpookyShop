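; BPC_Inventory is a player character inventory component that holds a collection of unique items.
; Add and remove functions check membership, broadcast OnItemAdded or OnItemRemoved on change, return success and print debug messages, though successful removal also prints "no item to remove".
; A lookup function reports whether an item is held, and the I key prints all item names.
; SwitchItem is an empty stub.
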(event Input|KeyboardEvents|DebugKeyI
  (params (Key :type Key%20Structure) (ActionValue :type Input%20Action%20Value%20Structure))
  (:Pressed
    (CallFunction|DebugItems)))

(fn TryAddItem
  (params (ItemToAdd :type Struct%20Item%20Structure%20%28by%20ref%29))
  (if (Utilities|Array|ContainsItem (Variables|Default|GetItems) ItemToAdd)
    (Development|PrintString "Item already in inventory")
    (return false)
    (else
      (Utilities|Array|Add (Variables|Default|GetItems) ItemToAdd)
      (Default|CallOnItemAdded ItemToAdd)
      (Development|PrintString "Item added to inventory")
      (return true))))

(fn TryRemoveItem
  (params (ItemToRemove :type Struct%20Item%20Structure%20%28by%20ref%29))
  (if (Utilities|Array|ContainsItem (Variables|Default|GetItems) ItemToRemove)
    (bind _returnvalue (Utilities|Array|RemoveItem (Variables|Default|GetItems) ItemToRemove))
    (Default|CallOnItemRemoved ItemToRemove)
    (Development|PrintString "no item to remove")
    (return _returnvalue)
    (else
      (Development|PrintString "no item to remove")
      (return false))))

(fn CheckforItem
  (params (ItemToCheck :type Struct%20Item%20Structure%20%28by%20ref%29))
  (return (Utilities|Array|ContainsItem (Variables|Default|GetItems) ItemToCheck)))

(fn DebugItems
  (for _array_element (Variables|Default|GetItems)
    (Development|PrintString (Utilities|String|ToString(Name) (.ItemName (Utilities|Struct|BreakStruct_Item _array_element))))))

(fn SwitchItem
  (params (ItemIndex :type Integer)))