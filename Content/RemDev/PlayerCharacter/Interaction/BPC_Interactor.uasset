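; Scene component that detects the interactable the player is looking at and triggers interaction with it.
; A looping timer runs a forward Visibility line trace and keeps the hit actor if it implements BPI_Interaction.
; Target changes send look started/ended interface messages and fire callbacks, though switching directly between interactables skips the ended callback.
; TryInteract forwards an interact message to the current target.
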(event Custom|CheckForInteractable
  (CallFunction|CheckforInteractables))

(event Custom|TryInteract
  (Class|BPIInteraction|Interact(Message) (Variables|Default|GetCurrentInteractableInSight)))

(event EventBeginPlay
  (Utilities|Time|SetTimerbyEvent (delegate Custom|CheckForInteractable) 0.2 true))

(fn CheckforInteractables
  (bind _returnvalue (Transformation|GetWorldLocation))
  (bind _outhit (Collision|LineTraceByChannel _returnvalue (+ _returnvalue (* (Math|Vector|GetForwardVector) (Variables|Default|GetInteractionDistance))) "TraceTypeQuery1" false 0 "None"))
  (bind _output_get (LocalVariables|SetCurrentActorInSight (.HitActor (Collision|BreakHitResult _outhit))))
  ;[1 0.5029 0] Does current actor in sight implements BPI Interaction?
  (if (Utilities|DoesObjectImplementInterface _output_get "/Game/RemDev/PlayerCharacter/Interaction/BPI_Interaction.BPI_Interaction_C")
    ;[1 0.5029 0] Does current Interactable in sight exist?
    (Utilities|IsValid (Variables|Default|GetCurrentInteractableInSight)
      (:Is%20Valid
        ;[1 0.5029 0] Is current actor in sight same as current interactable in sight?
        (if (== (LocalVariables|GetCurrentActorInSight) (Variables|Default|GetCurrentInteractableInSight))
          (Development|PrintString "Same interactable in sight")
          (else
            (Class|BPIInteraction|LookEnded(Message) (Variables|Default|GetCurrentInteractableInSight))
            (bind _output_get_2 (Variables|Default|SetCurrentInteractableInSight (LocalVariables|GetCurrentActorInSight)))
            (Class|BPIInteraction|LookStarted(Message) _output_get_2)
            (Default|CallOnLookStartedCallback _output_get_2))))
      (:Is%20Not%20Valid
        (bind _output_get_3 (Variables|Default|SetCurrentInteractableInSight (LocalVariables|GetCurrentActorInSight)))
        (Class|BPIInteraction|LookStarted(Message) _output_get_3)
        (Default|CallOnLookStartedCallback (Variables|Default|GetCurrentInteractableInSight))))
    (else
      ;[1 0.5029 0] previous interactable on sight exists?
      (Utilities|IsValid (Variables|Default|GetCurrentInteractableInSight)
        (:Is%20Valid
          (Class|BPIInteraction|LookEnded(Message) (Variables|Default|GetCurrentInteractableInSight))
          (Default|CallOnLookEndedCallback (Variables|Default|GetCurrentInteractableInSight)))
        (:Is%20Not%20Valid
          _))
      (Variables|Default|SetCurrentInteractableInSight 0)
      (Default|CallOnInteractableNullCallback))))