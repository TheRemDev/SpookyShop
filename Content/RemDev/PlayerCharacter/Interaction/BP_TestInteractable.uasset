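; BP_TestInteractable is a test actor that gives visual feedback for the player interaction events LookStarted, LookEnded and Interact.
; On BeginPlay it creates a dynamic material instance on its mesh, whose Color parameter turns blue while looked at and grey when the look ends.
; Interact pulses the root's scale slightly up and back, using one timeline forward and a second played in reverse once the first finishes.
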(event EventLookEnded
  (Rendering|Material|SetVectorParameterValue (Variables|Default|GetTestMaterialInstance) "Color" "(R=0.500000,G=0.500000,B=0.500000,A=1.000000)" :!class /Script/Engine.MaterialInstanceDynamic))

(event EventLookStarted
  (Rendering|Material|SetVectorParameterValue (Variables|Default|GetTestMaterialInstance) "Color" "(R=0.000000,G=0.420181,B=1.000000,A=1.000000)" :!class /Script/Engine.MaterialInstanceDynamic))

(event EventInteract
  (bind _alpha (Timeline|Timeline PlayFromStart)
    (:Update
      (Transformation|SetRelativeScale3D (Variables|Default|GetDefaultSceneRoot) (Math|Vector|Lerp(Vector) "1.000000,1.000000,1.000000" "1.150000,1.150000,1.150000" _alpha)))
    (:Finished
      (bind _alpha_2 (Timeline|Timeline_0 ReverseFromEnd)
        (:Update
          (Transformation|SetRelativeScale3D (Variables|Default|GetDefaultSceneRoot) (Math|Vector|Lerp(Vector) "1.000000,1.000000,1.000000" "1.150000,1.150000,1.150000" _alpha_2)))))))

(event EventBeginPlay
  ;[1 1 1] Init Material Instance for Testing
  (bind _returnvalue (Rendering|Material|CreateDynamicMaterialInstance (Variables|Default|GetMesh) 0 "/Game/RemDev/PlayerCharacter/TestMaterials/Mat_TestInteractable.Mat_TestInteractable" "None" :!class /Script/Engine.PrimitiveComponent))
  (bind _output_get (Variables|Default|SetTestMaterialInstance _returnvalue))
  (Rendering|Material|SetMaterial (Variables|Default|GetMesh) 0 _output_get))

(fn ConstructionScript)