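; BPC_Health is a health component in the player character folder that tracks current health against a maximum.
; Health starts at MaxHealth on BeginPlay, and AddHealth and RemoveHealth adjust it, clamped between zero and that maximum.
; Each change fires an added or removed event dispatcher, and removal that leaves health at zero also fires the depleted one.
; GetHealth exposes the current value.
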(event EventBeginPlay
  ;[1 1 1] Init Health
  (Variables|Default|SetHealth (Variables|Default|GetMaxHealth)))

(event EventAddHealth
  (params (HealthToAdd :type Integer))
  ;[0.769 1 0.09549] Add Remove Health
  (Variables|Default|SetHealth (Math|Integer|Clamp(Integer) (+ (Variables|Default|GetHealth) HealthToAdd) 0 (Variables|Default|GetMaxHealth)))
  (Default|CallOnHealthAdded))

(event EventRemoveHealth
  (params (HealthToRemove :type Integer))
  ;[0.769 1 0.09549] Add Remove Health
  (bind _output_get (Variables|Default|SetHealth (Math|Integer|Clamp(Integer) (- (Variables|Default|GetHealth) HealthToRemove) 0 (Variables|Default|GetMaxHealth))))
  (if (<= _output_get 0)
    (Default|CallOnHealthRemoved)
    (Default|CallOnHealthDepletead)
    (else
      (Default|CallOnHealthRemoved))))

(fn GetHealth
  (return (Variables|Default|GetHealth)))