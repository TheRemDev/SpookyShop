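; BP_TestHealth is a test actor that reacts to damage through its BPC_Health component.
; On BeginPlay it applies a dynamic instance of Mat_TestInteractable to its static mesh.
; Health removal briefly flashes the material's Color red before restoring grey, and health depletion destroys the actor.
; GetHealth is a stub that returns zero rather than reading the component.
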(event OnHealthRemoved(BPC_Health)
  (Rendering|Material|SetVectorParameterValue (Variables|Default|GetMatInstanceRef) "Color" "(R=1.000000,G=0.000000,B=0.000000,A=1.000000)" :!class /Script/Engine.MaterialInstanceDynamic)
  (Utilities|FlowControl|Delay 0.1)
  (Rendering|Material|SetVectorParameterValue (Variables|Default|GetMatInstanceRef) "Color" "(R=0.500000,G=0.500000,B=0.500000,A=1.000000)" :!class /Script/Engine.MaterialInstanceDynamic))

(event OnHealthDepletead(BPC_Health)
  (Actor|DestroyActor))

(event EventBeginPlay
  (bind _returnvalue (Rendering|Material|CreateDynamicMaterialInstance "/Game/RemDev/PlayerCharacter/TestMaterials/Mat_TestInteractable.Mat_TestInteractable" "None" "None" :!class /Script/Engine.KismetMaterialLibrary))
  (bind _output_get (Variables|Default|SetMatInstanceRef _returnvalue))
  (Rendering|Material|SetMaterial (Variables|Default|GetStaticMesh) 0 _output_get))

(fn ConstructionScript)

(fn GetHealth
  (return 0))