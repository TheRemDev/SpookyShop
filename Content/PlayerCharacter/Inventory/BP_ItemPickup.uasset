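; BP_ItemPickup is a world item pickup that the player collects into their inventory by interacting with it.
; The construction script looks up the selected row in DT_Items and sets the mesh from it, so each placed instance shows its item.
; On Interact it passes that row to the player's BPC_Inventory component through TryAddItem and destroys itself only if the add succeeds.
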(event EventBeginPlay
  (|CallParentFunction) ; This node is disabled and will not be called.\nDrag off pins to build functionality.
)

(event EventInteract
  (bind _returnvalue (Game|GetPlayerCharacter 0))
  (bind _returnvalue_2 (Actor|GetComponentbyClass _returnvalue "/Game/PlayerCharacter/Inventory/BPC_Inventory.BPC_Inventory_C"))
  (Utilities|IsValid _returnvalue_2
    (:Is%20Valid
      (bind _returnvalue_3 (Utilities|GetDataTableRow "/Game/PlayerCharacter/Inventory/DT_Items.DT_Items" (.rowname (Variables|Default|GetItemSelector)))
        (:then
          (bind _success_ (Default|TryAddItem _returnvalue_2 _returnvalue_3))
          (if _success_
            (Actor|DestroyActor)))))))

(fn ConstructionScript
  (|CallParentFunction)
  (bind _returnvalue (Utilities|GetDataTableRow "/Game/PlayerCharacter/Inventory/DT_Items.DT_Items" (.rowname (Variables|Default|GetItemSelector)))
    (:then
      (Components|StaticMesh|SetStaticMesh (Variables|Character|GetMesh) (.Mesh (Utilities|Struct|BreakStruct_Item _returnvalue))))))