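; BP_ItemCheckTest is a test pad that shows whether an overlapping actor's inventory holds a required item.
; On box overlap it looks up ItemRequired in DT_Items and passes the row to the actor's BPC_Inventory CheckForItem.
; A dynamic material on the floor mesh turns green or red for the result and grey when the actor leaves.
; The construction script labels the pad with the required item's row name.
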(event OnComponentBeginOverlap(BoxCollider)
  (params (OverlappedComponent :type Primitive%20Component%20Object%20Reference) (OtherActor :type Actor%20Object%20Reference) (OtherComp :type Primitive%20Component%20Object%20Reference) (OtherBodyIndex :type Integer) (bFromSweep :type Boolean) (SweepResult :type Hit%20Result%20Structure%20%28by%20ref%29))
  (bind _returnvalue (Actor|GetComponentbyClass OtherActor "/Game/PlayerCharacter/Inventory/BPC_Inventory.BPC_Inventory_C"))
  (bind _materialinstanceref (Variables|Default|GetMaterialInstanceRef))
  (Utilities|IsValid _returnvalue
    (:Is%20Valid
      (bind _returnvalue_2 (Utilities|GetDataTableRow "/Game/PlayerCharacter/Inventory/DT_Items.DT_Items" (.rowname (Variables|Default|GetItemRequired)))
        (:then
          (bind _containsitem_ (Default|CheckforItem _returnvalue _returnvalue_2))
          (if _containsitem_
            (Rendering|Material|SetVectorParameterValue _materialinstanceref "Color" "(R=0.000000,G=1.000000,B=0.000000,A=1.000000)" :!class /Script/Engine.MaterialInstanceDynamic)
            (else
              (Rendering|Material|SetVectorParameterValue _materialinstanceref "Color" "(R=1.000000,G=0.000000,B=0.000000,A=1.000000)" :!class /Script/Engine.MaterialInstanceDynamic))))))))

(event OnComponentEndOverlap(BoxCollider)
  (params (OverlappedComponent :type Primitive%20Component%20Object%20Reference) (OtherActor :type Actor%20Object%20Reference) (OtherComp :type Primitive%20Component%20Object%20Reference) (OtherBodyIndex :type Integer))
  (Utilities|IsValid (Actor|GetComponentbyClass OtherActor "/Game/PlayerCharacter/Inventory/BPC_Inventory.BPC_Inventory_C")
    (:Is%20Valid
      (Rendering|Material|SetVectorParameterValue (Variables|Default|GetMaterialInstanceRef) "Color" "(R=0.500000,G=0.500000,B=0.500000,A=1.000000)" :!class /Script/Engine.MaterialInstanceDynamic))))

(event EventBeginPlay
  (bind _returnvalue (Rendering|Material|CreateDynamicMaterialInstance (Variables|Default|GetFloorMesh) 0 "/Game/PlayerCharacter/TestMaterials/Mat_TestInteractable.Mat_TestInteractable" "None" :!class /Script/Engine.PrimitiveComponent))
  (bind _output_get (Variables|Default|SetMaterialInstanceRef _returnvalue))
  (Rendering|Material|SetMaterial (Variables|Default|GetFloorMesh) 0 _output_get))

(fn ConstructionScript
  (Rendering|Components|TextRender|SetText (Variables|Default|GetTextRender) (Utilities|Text|ToText(Name) (.rowname (Variables|Default|GetItemRequired)))))